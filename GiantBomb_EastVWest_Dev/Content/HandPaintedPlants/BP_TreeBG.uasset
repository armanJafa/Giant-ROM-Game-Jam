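; BP_TreeBG is a tree actor, apparently for background scenery, that varies the size of its four tree components at runtime.
; On BeginPlay it passes each tree to ScaleTreeRandom, which sets a random relative scale within SizeRangeMin and SizeRangeMax.
; Y and Z are rolled independently while X stays at 1, so proportions vary as well as size.
; The construction script is empty, so the variation appears only in play.
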(event EventBeginPlay
  (CallFunction|ScaleTreeRandom (Variables|Default|GetTree))
  (CallFunction|ScaleTreeRandom (Variables|Default|GetTree2))
  (CallFunction|ScaleTreeRandom (Variables|Default|GetTree3))
  (CallFunction|ScaleTreeRandom (Variables|Default|GetTree4)))

(fn ConstructionScript)

(fn ScaleTreeRandom
  (params (Mesh :type Scene%20Component%20Object%20Reference))
  (bind _sizerangemax (Variables|Default|GetSizeRangeMax))
  (bind _sizerangemin (Variables|Default|GetSizeRangeMin))
  (bind _returnvalue (Math|Random|RandomFloatinRange _sizerangemin _sizerangemax))
  (Transformation|SetRelativeScale3D Mesh (Math|Vector|MakeVector 1.0 _returnvalue _returnvalue)))